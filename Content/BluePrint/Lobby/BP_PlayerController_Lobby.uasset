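; Lobby player controller that creates the lobby UI and switches it between lobby and room views.
; On BeginPlay, except on dedicated servers, it adds the W_RealLobby widget to the viewport, shows the cursor and sets UI-only input.
; OnUpdatePlayerState reads THPlayerState_Lobby and uses LobbyWidgetSwitcher to show either the lobby or the player's room, which it renders.
; SetNickname is an empty stub.
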(event EventOnUpdatePlayerState
  (bind _lobbywidgetswitcher (Variables|Default|GetLobbyWidgetSwitcher))
  (bind _widgetswitcher (Variables|/Game/BluePrint/Lobby/W_LobbyWidgetSwitcher.W_LobbyWidgetSwitcher_C|GetWidgetSwitcher _lobbywidgetswitcher))
  (bind _w_room (Variables|/Game/BluePrint/Lobby/W_LobbyWidgetSwitcher.W_LobbyWidgetSwitcher_C|GetW_Room _lobbywidgetswitcher))
  (bind _asthplayer_state_lobby (Utilities|Casting|CastToTHPlayerState_Lobby (Variables|Default|GetPlayerState)))
  (bind _returnvalue (Class|THPlayerStateLobby|IsPlayerinRoom _asthplayer_state_lobby))
  (if _returnvalue
    (Class|WidgetSwitcher|SetActiveWidget _widgetswitcher _w_room)
    (bind _returnvalue_2 (Class|THPlayerStateLobby|GetPlayerRoom _asthplayer_state_lobby))
    (Class|THWidgetRoom|RenderRoom _w_room _returnvalue_2)
    (else
      (Class|WidgetSwitcher|SetActiveWidget _widgetswitcher (Variables|/Game/BluePrint/Lobby/W_LobbyWidgetSwitcher.W_LobbyWidgetSwitcher_C|GetW_Lobby _lobbywidgetswitcher)))))

(event EventBeginPlay
  (bind _self self)
  (if (not (Networking|IsDedicatedServer))
    (Utilities|FlowControl|Sequence
      (:then_0
        (bind _returnvalue (UserInterface|CreateWidget "/Game/BluePrint/Lobby/W_RealLobby.W_RealLobby_C"))
        (bind _output_get (Variables|Default|SetReadLobby _returnvalue))
        (UserInterface|Viewport|AddtoViewport _output_get 0))
      (:then_1
        (Variables|/Script/Engine.PlayerController|SetbShowMouseCursor _self true)
        (Input|SetInputModeUIOnly _self 0 "DoNotLock" false)))))

(fn ConstructionScript)

(fn SetNickname
  (params (InputText :type Text)))